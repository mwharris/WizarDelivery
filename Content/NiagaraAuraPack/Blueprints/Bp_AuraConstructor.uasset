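; Configurable aura effect actor that plays one of twelve Niagara auras in begin, loop and end phases.
; The construction script assigns the systems for the chosen Aura to Start, Middle, End and a Preview component, which is destroyed at BeginPlay.
; Spawn runs automatically unless ManuallySpawn is set, playing Start briefly before switching to Middle.
; Unless Infinity is set, Middle gives way to End after Time.
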(event Custom|Spawn
  (Components|Activation|Activate (Variables|Default|GetStart) false)
  (Utilities|FlowControl|Delay 1.0)
  (Components|Activation|Deactivate (Variables|Default|GetStart))
  (Components|Activation|Activate (Variables|Default|GetMiddle) true)
  (if (not (Variables|Default|GetInfinity))
    (Utilities|FlowControl|Delay (Variables|Default|GetTime))
    (Components|Activation|Activate (Variables|Default|GetEnd) false)
    (Components|Activation|Deactivate (Variables|Default|GetMiddle))))

(event EventBeginPlay
  (if (Variables|Default|GetManuallySpawn)
    _
    (else
      (CallFunction|Spawn)))
  (Components|DestroyComponent (Variables|Default|GetPreview)))

(fn ConstructionScript
  (bind _aura (Variables|Default|GetAura))
  (bind _returnvalue (Utilities|Select :Index _aura :NewEnumerator0 "/Game/NiagaraAuraPack/Niagara/NiagaraSystems/NS_aura1.NS_aura1" :NewEnumerator1 "/Game/NiagaraAuraPack/Niagara/NiagaraSystems/NS_aura2.NS_aura2" :NewEnumerator2 "/Game/NiagaraAuraPack/Niagara/NiagaraSystems/NS_aura3.NS_aura3" :NewEnumerator3 "/Game/NiagaraAuraPack/Niagara/NiagaraSystems/NS_aura4.NS_aura4" :NewEnumerator4 "/Game/NiagaraAuraPack/Niagara/NiagaraSystems/NS_aura5.NS_aura5" :NewEnumerator5 "/Game/NiagaraAuraPack/Niagara/NiagaraSystems/NS_aura6.NS_aura6" :NewEnumerator6 "/Game/NiagaraAuraPack/Niagara/NiagaraSystems/NS_aura7.NS_aura7" :NewEnumerator7 "/Game/NiagaraAuraPack/Niagara/NiagaraSystems/NS_aura8.NS_aura8" :NewEnumerator8 "/Game/NiagaraAuraPack/Niagara/NiagaraSystems/NS_aura9.NS_aura9" :NewEnumerator9 "/Game/NiagaraAuraPack/Niagara/NiagaraSystems/NS_aura10.NS_aura10" :NewEnumerator10 "/Game/NiagaraAuraPack/Niagara/NiagaraSystems/NS_aura11.NS_aura11" :NewEnumerator11 "/Game/NiagaraAuraPack/Niagara/NiagaraSystems/NS_aura12.NS_aura12"))
  (Class|NiagaraComponent|SetAsset (Variables|Default|GetPreview) _returnvalue)
  (Class|NiagaraComponent|SetAsset (Variables|Default|GetMiddle) _returnvalue)
  (Class|NiagaraComponent|SetAsset (Variables|Default|GetStart) (Utilities|Select :Index _aura :NewEnumerator0 "/Game/NiagaraAuraPack/Niagara/NiagaraSystems/NS_aura1_begin.NS_aura1_begin" :NewEnumerator1 "/Game/NiagaraAuraPack/Niagara/NiagaraSystems/NS_aura2_begin.NS_aura2_begin" :NewEnumerator2 "/Game/NiagaraAuraPack/Niagara/NiagaraSystems/NS_aura3_begin.NS_aura3_begin" :NewEnumerator3 "/Game/NiagaraAuraPack/Niagara/NiagaraSystems/NS_aura4_begin.NS_aura4_begin" :NewEnumerator4 "/Game/NiagaraAuraPack/Niagara/NiagaraSystems/NS_aura5_begin.NS_aura5_begin" :NewEnumerator5 "/Game/NiagaraAuraPack/Niagara/NiagaraSystems/NS_aura6_begin.NS_aura6_begin" :NewEnumerator6 "/Game/NiagaraAuraPack/Niagara/NiagaraSystems/NS_aura7_begin.NS_aura7_begin" :NewEnumerator7 "/Game/NiagaraAuraPack/Niagara/NiagaraSystems/NS_aura8_begin.NS_aura8_begin" :NewEnumerator8 "/Game/NiagaraAuraPack/Niagara/NiagaraSystems/NS_aura9_begin.NS_aura9_begin" :NewEnumerator9 "/Game/NiagaraAuraPack/Niagara/NiagaraSystems/NS_aura10_begin.NS_aura10_begin" :NewEnumerator10 "/Game/NiagaraAuraPack/Niagara/NiagaraSystems/NS_aura11_begin.NS_aura11_begin" :NewEnumerator11 "/Game/NiagaraAuraPack/Niagara/NiagaraSystems/NS_aura12_begin.NS_aura12_begin"))
  (Class|NiagaraComponent|SetAsset (Variables|Default|GetEnd) (Utilities|Select :Index _aura :NewEnumerator0 "/Game/NiagaraAuraPack/Niagara/NiagaraSystems/NS_aura1_end.NS_aura1_end" :NewEnumerator1 "/Game/NiagaraAuraPack/Niagara/NiagaraSystems/NS_aura2_end.NS_aura2_end" :NewEnumerator2 "/Game/NiagaraAuraPack/Niagara/NiagaraSystems/NS_aura3_end.NS_aura3_end" :NewEnumerator3 "/Game/NiagaraAuraPack/Niagara/NiagaraSystems/NS_aura4_end.NS_aura4_end" :NewEnumerator4 "/Game/NiagaraAuraPack/Niagara/NiagaraSystems/NS_aura5_end.NS_aura5_end" :NewEnumerator5 "/Game/NiagaraAuraPack/Niagara/NiagaraSystems/NS_aura6_end.NS_aura6_end" :NewEnumerator6 "/Game/NiagaraAuraPack/Niagara/NiagaraSystems/NS_aura7_end.NS_aura7_end" :NewEnumerator7 "/Game/NiagaraAuraPack/Niagara/NiagaraSystems/NS_aura8_end.NS_aura8_end" :NewEnumerator8 "/Game/NiagaraAuraPack/Niagara/NiagaraSystems/NS_aura9_end.NS_aura9_end" :NewEnumerator9 "/Game/NiagaraAuraPack/Niagara/NiagaraSystems/NS_aura10_end.NS_aura10_end" :NewEnumerator10 "/Game/NiagaraAuraPack/Niagara/NiagaraSystems/NS_aura11_end.NS_aura11_end" :NewEnumerator11 "/Game/NiagaraAuraPack/Niagara/NiagaraSystems/NS_aura12_end.NS_aura12_end")))